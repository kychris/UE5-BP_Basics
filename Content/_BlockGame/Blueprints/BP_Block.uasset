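; BP_Block is a placeable block in the block game that can be broken over time.
; On BeginPlay it creates a dynamic material instance and sets the destroy timeline's play rate from DestroyRate.
; StartDestroy animates the material's DestroyAmount through the timeline, while StopDestroy cancels and resets it.
; When the timeline finishes, the block reports its class and transform to GI_BlockGame's RemoveBlock, then destroys itself.
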(event Custom|StartDestroy
  (bind _defaultsceneroot (Variables|Default|GetDefaultSceneRoot))
  (bind _destroyamount (Timeline|Destroy%20Timeline PlayFromStart)
    (:Update
      (Rendering|Material|SetScalarParameterValue (Variables|Default|GetBlockMat) "DestroyAmount" _destroyamount :!class /Script/Engine.MaterialInstanceDynamic))
    (:Finished
      (Default|RemoveBlock (.AsGI%20Block%20Game (Utilities|Casting|CastToGI_BlockGame (Game|GetGameInstance))) (Utilities|Struct|MakeST_BlockData (Utilities|GetClass self) (Transformation|GetWorldLocation _defaultsceneroot) (Transformation|GetWorldRotation _defaultsceneroot)))
      (Actor|DestroyActor))))

(event Custom|StopDestroy
  (bind _defaultsceneroot (Variables|Default|GetDefaultSceneRoot))
  (Rendering|Material|SetScalarParameterValue (Variables|Default|GetBlockMat) "DestroyAmount" 0.0 :!class /Script/Engine.MaterialInstanceDynamic) ; Reset material destroy parameter
  (bind _destroyamount (Timeline|Destroy%20Timeline Stop)
    (:Update
      (Rendering|Material|SetScalarParameterValue (Variables|Default|GetBlockMat) "DestroyAmount" _destroyamount :!class /Script/Engine.MaterialInstanceDynamic))
    (:Finished
      (Default|RemoveBlock (.AsGI%20Block%20Game (Utilities|Casting|CastToGI_BlockGame (Game|GetGameInstance))) (Utilities|Struct|MakeST_BlockData (Utilities|GetClass self) (Transformation|GetWorldLocation _defaultsceneroot) (Transformation|GetWorldRotation _defaultsceneroot)))
      (Actor|DestroyActor))))

(event EventBeginPlay
  (bind _block (Variables|Default|GetBlock))
  (bind _returnvalue (Rendering|Material|CreateDynamicMaterialInstance _block 0 (Rendering|Material|GetMaterial _block 0) "None" :!class /Script/Engine.PrimitiveComponent))
  (Variables|Default|SetBlockMat _returnvalue)
  (Components|Timeline|SetPlayRate (Variables|Default|GetDestroy%20Timeline) (Variables|Default|GetDestroyRate)))

(fn ConstructionScript)