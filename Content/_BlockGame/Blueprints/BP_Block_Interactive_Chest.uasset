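; Interactive chest block for the block game, whose lid opens and closes on interaction.
; On BeginPlay the Top mesh copies the material of the base Block.
; Interact uses a FlipFlop to play or reverse the OpenCloseChest timeline, which drives the Pivot component's pitch to swing the lid.
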(event EventBeginPlay
  (|CallParentFunction)
  (Rendering|Material|SetMaterial (Variables|Default|GetTop) 0 (Rendering|Material|GetMaterial (Variables|Default|GetBlock) 0)))

(event EventInteract
  (Utilities|FlowControl|FlipFlop
    (:A
      (bind _openamount (Timeline|OpenCloseChest Play)
        (:Update
          (Transformation|SetRelativeRotation (Variables|Default|GetPivot) (Math|Rotator|MakeRotator 0.0 _openamount 0.0) false false))))
    (:B
      (Timeline|OpenCloseChest Reverse))))

(fn ConstructionScript
  (|CallParentFunction))